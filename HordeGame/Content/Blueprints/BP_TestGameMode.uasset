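; Test game mode that rewards kills with score and spawns BP_TrackerBot enemies.
; On BeginPlay it binds to OnActorKilled, adding points to the killer's SPlayerState when the victim is a non-player pawn and printing the new score.
; SpawnNewBot runs the EQS_FindSpawnLocation query, picking from the best 25%, then spawns a bot with a debug sphere at each returned location.
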(event `self.ReceiveBeginPlay`
  (add `self.OnActorKilled` (delegate `OnActorKilled_Event`)))

(event `OnActorKilled_Event` :!signature `self.OnActorKilled`
  (params (VictimActor :type "Actor Object Reference") (KillerActor :type "Actor Object Reference") (KillerController :type "Controller Object Reference"))
  ;[1 1 1] Do not reward killing fellow players
  (bind _aspawn (cast `Pawn` VictimActor))
  (if (not (`Pawn.IsPlayerControlled` _aspawn))
    ;[1 1 1] Reward the killer with some points
    (bind _assplayer_state (cast `SPlayerState` (`Pawn.PlayerState` (`Controller.K2_GetPawn` KillerController))))
    (`SPlayerState.AddScore` _assplayer_state 20.0)
    (`KismetSystemLibrary.PrintString` (`KismetStringLibrary.Conv_DoubleToString` (`PlayerState.Score` _assplayer_state)) true true (struct :`R` 0.129164 :`G` 1.0 :`B` 0.226884 :`A` 1.0))))

(event `self.SpawnNewBot`
  (bind _returnvalue (`EnvQueryManager.RunEQSQuery` "/Game/Blueprints/EQS_FindSpawnLocation.EQS_FindSpawnLocation" self "RandomBest25Pct"))
  (add `EnvQueryInstanceBlueprintWrapper.OnQueryFinishedEvent` _returnvalue (delegate `CustomEvent_0`)))

(event `CustomEvent_0`
  (params (QueryInstance :type "EnvQueryInstanceBlueprintWrapper Object Reference") (QueryStatus :type "EEnvQueryStatus Enum" :default "Processing"))
  (switch `EEnvQueryStatus` QueryStatus
    (:`Success`
      (for _array_element (`EnvQueryInstanceBlueprintWrapper.GetResultsAsLocations` QueryInstance)
        (`KismetSystemLibrary.DrawDebugSphere` _array_element 50.0 12 (struct :`R` 1.0 :`G` 0.848041 :`A` 1.0) 2.0 2.0)
        (`|SpawnActorFromClass` "/Game/Blueprints/BP_TrackerBot.BP_TrackerBot_C" (`KismetMathLibrary.MakeTransform` _array_element) "AdjustIfPossibleButDontSpawnIfColliding" "OverrideRootScale" null null)))))

(fn `UserConstructionScript`)
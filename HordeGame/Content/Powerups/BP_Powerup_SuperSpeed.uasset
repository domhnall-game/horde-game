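; Super speed powerup that doubles the affected actor's walk speed while active.
; OnActivated and OnExpired call their parent implementations, then double or halve MaxWalkSpeed on that actor's CharacterMovementComponent.
; Both pass the resulting value to the ReplicateMaxWalkSpeed event, which sets it again on the actor's movement component.
; The change is relative, with no original speed stored.
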(event `self.OnActivated`
  (bind _activeforactor (`self.ActiveForActor`))
  (bind _returnvalue (`self.GetComponentByClass` _activeforactor "/Script/Engine.CharacterMovementComponent"))
  (`/Engine/EditorBlueprintResources/StandardMacros.IsValid` _activeforactor
    (:`Is Valid`
      (`parent.OnActivated`)
      (`/Engine/EditorBlueprintResources/StandardMacros.IsValid` _returnvalue
        (:`Is Valid`
          (bind _output_get (set `CharacterMovementComponent.MaxWalkSpeed` (* 2 (`CharacterMovementComponent.MaxWalkSpeed` _returnvalue)) _returnvalue))
          (`self.ReplicateMaxWalkSpeed` _output_get (`self.ActiveForActor`)))))))

(event `self.OnExpired`
  (bind _activeforactor (`self.ActiveForActor`))
  (bind _returnvalue (`self.GetComponentByClass` _activeforactor "/Script/Engine.CharacterMovementComponent"))
  (`/Engine/EditorBlueprintResources/StandardMacros.IsValid` _activeforactor
    (:`Is Valid`
      (`parent.OnExpired`)
      (`/Engine/EditorBlueprintResources/StandardMacros.IsValid` _returnvalue
        (:`Is Valid`
          (bind _output_get (set `CharacterMovementComponent.MaxWalkSpeed` (/ (`CharacterMovementComponent.MaxWalkSpeed` _returnvalue) 2.0) _returnvalue))
          (`self.ReplicateMaxWalkSpeed` _output_get (`self.ActiveForActor`)))))))

(event `ReplicateMaxWalkSpeed`
  (params (NewMaxWalkSpeed :type "Float (double-precision)") (ActiveForActor :type "Actor Object Reference"))
  (set `CharacterMovementComponent.MaxWalkSpeed` NewMaxWalkSpeed (`self.GetComponentByClass` ActiveForActor "/Script/Engine.CharacterMovementComponent")))

(fn `UserConstructionScript`)